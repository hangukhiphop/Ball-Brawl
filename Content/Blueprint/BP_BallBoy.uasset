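; BP_BallBoy is a 2D ball boy sprite that switches its animation according to directional input.
; It adds a Paper Flipbook component at BeginPlay, then the horizontal and vertical axis events set directional BlueBoy run flipbooks from the input's sign.
; Both events share a NOR check that plays the Dizzy flipbook when input is zero.
; The graph only changes animation and applies no movement.
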(event EventBeginPlay
  (bind _returnvalue (AddComponent|AddPaperFlipbookComponent false)))

(event Input|AxisEvents|InputAxisMove_Horizontal
  (params (AxisValue :type Float%20%28single-precision%29))
  (bind _returnvalue (!= AxisValue 0.0))
  (if _returnvalue
    (if (> AxisValue 0.0)
      (Sprite|SetFlipbook (stale EventBeginPlay _returnvalue) "/Game/Animations/BlueBoy_Run_Right.BlueBoy_Run_Right")
      (else
        (Sprite|SetFlipbook (stale EventBeginPlay _returnvalue) "/Game/Animations/BlueBoy_Run_Left.BlueBoy_Run_Left")))
    (elif (Math|Boolean|NORBoolean _returnvalue (!= (stale Input|AxisEvents|InputAxisMove_Vertical AxisValue) 0.0))
      (Sprite|SetFlipbook (stale EventBeginPlay _returnvalue) "/Game/Animations/BlueBoy_Dizzy.BlueBoy_Dizzy"))))

(event Input|AxisEvents|InputAxisMove_Vertical
  (params (AxisValue :type Float%20%28single-precision%29))
  (bind _returnvalue (!= AxisValue 0.0))
  (if _returnvalue
    (if (> AxisValue 0.0)
      (Sprite|SetFlipbook (stale EventBeginPlay _returnvalue) "/Game/Animations/BlueBoy_Run_Up.BlueBoy_Run_Up")
      (else
        (Sprite|SetFlipbook (stale EventBeginPlay _returnvalue) "/Game/Animations/BlueBoy_Run_Down.BlueBoy_Run_Down")))
    (elif (Math|Boolean|NORBoolean (!= (stale Input|AxisEvents|InputAxisMove_Horizontal AxisValue) 0.0) _returnvalue)
      (Sprite|SetFlipbook (stale EventBeginPlay _returnvalue) "/Game/Animations/BlueBoy_Dizzy.BlueBoy_Dizzy"))))

(fn ConstructionScript)